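; BP_Catapult is a physics-driven catapult with Shoot and ReplayCatapult (reload) events.
; Shoot makes the Sphere component heavy and Replei light through mass overrides, and reload shifts the weight back toward Replei.
; After a delay, reload spawns a new BP_Ball at a hardcoded world location.
; The CanIsShoot flag alternates the two actions, flipping only after each delay.
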(event Custom|Shoot
  ;[1 1 1] Реализуйте механику выстрела
  (Development|PrintString "Catapult shot!")
  (if (Variables|Default|GetCanIsShoot)
    (Class|PrimitiveComponent|SetMassOverrideinKg (Variables|Default|GetSphere) "None" 3e+03 true)
    (Class|PrimitiveComponent|SetMassOverrideinKg (Variables|Default|GetReplei) "None" 2.0 true)
    (Utilities|FlowControl|Delay 3.0)
    (Variables|Default|SetCanIsShoot false)))

(event Custom|ReplayCatapult
  (if (not (Variables|Default|GetCanIsShoot))
    (Class|PrimitiveComponent|SetMassOverrideinKg (Variables|Default|GetSphere) "None" 2.0 true)
    (Class|PrimitiveComponent|SetMassOverrideinKg (Variables|Default|GetReplei) "None" 5e+02 true)
    (Utilities|FlowControl|Delay 3.0)
    (Game|SpawnActorfromClass "/Game/HW_03/Blueprints/Cannonball/BP_Ball.BP_Ball_C" (Math|Transform|MakeTransform "670.000000,1723.000000,234.000000") "Undefined" "MultiplyWithRoot" 0 0)
    (Variables|Default|SetCanIsShoot true)))

(fn ConstructionScript)